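; BP_UpdateOnTickExample is an example actor that animates a procedural cave by rebuilding it every tick while the player pawn is within range.
; Update rotates four pivots to give the spline organic motion, then gathers world locations from the root and four mover components.
; It passes those points, with meshes and light settings, to its BP_ProceduralCave child actor through VariablesSetup.
; The construction script also runs Update.
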(event EventTick
  (params (DeltaSeconds :type Float%20%28single-precision%29))
  (Utilities|IsValid (Game|Player|GetPlayerPawn 0)
    (:Is%20Valid
      (if (< (Math|Vector|Distance(Vector) (Transformation|GetActorLocation) (Transformation|GetActorLocation (Game|Player|GetPlayerPawn 0))) 3e+04)
        (CallFunction|Update)))))

(fn ConstructionScript
  (CallFunction|Update))

(fn Update
  ;[1 1 1] These rotations produce the organic movement of the spline
  (Transformation|AddRelativeRotation (Variables|Default|GetPivot1) "0.000000,7.000000,1.000000" false false)
  (Transformation|AddRelativeRotation (Variables|Default|GetPivot2) "0.000000,9.000000,3.000000" false false)
  (Transformation|AddRelativeRotation (Variables|Default|GetPivot3) "0.000000,5.000000,2.000000" false false)
  (Transformation|AddRelativeRotation (Variables|Default|GetPivot4) "0.000000,2.000000,6.000000" false false)
  (Variables|Default|SetCurrentPointLocations (Utilities|Array|MakeArray (Transformation|GetWorldLocation (Variables|Default|GetDefaultSceneRoot)) (Transformation|GetWorldLocation (Variables|Default|GetMover1)) (Transformation|GetWorldLocation (Variables|Default|GetMover2)) (Transformation|GetWorldLocation (Variables|Default|GetMover3)) (Transformation|GetWorldLocation (Variables|Default|GetMover4))))
  (bind _asbp_procedural_cave (Utilities|Casting|CastToBP_ProceduralCave (Variables|/Script/Engine.ChildActorComponent|GetChildActor (Variables|Default|GetChildActor))))
  (Default|VariablesSetup _asbp_procedural_cave (Variables|Default|GetCurrentPointLocations) true (Variables|Default|GetMeshes) 1.0 0 false 5e+02 0.8 0 false 1e+03 1 1 "/Game/ProceduralCaves/CustomMeshes/SM_HollowCylinderSmooth.SM_HollowCylinderSmooth" (Utilities|Array|MakeArray "/Engine/EditorMaterials/LevelGridMaterial2.LevelGridMaterial2") "NoCollision" "ECC_WorldStatic" true 9999.0 "(R=1.000000,G=0.000000,B=0.000000,A=1.000000)" 0.5 1.0 0.0 true))