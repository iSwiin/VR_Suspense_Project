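; Handler actor that drives a BP_ProceduralCave child actor and exposes functions to alter or reset the cave.
; Reset, run from the construction script, restores default control points, width and seed.
; Change offsets one point, adjusts the clamped width and optionally replaces the seed.
; Both convert child-relative points to world space, then pass them with fixed mesh and light settings to the cave's VariablesSetup.
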(fn ConstructionScript
  (CallFunction|Reset))

(fn Change
  (params (Point :type Integer) (AddLocation :type Vector) (WidthChange :type Float%20%28double-precision%29) (UseNewSeeed :type Boolean) (NewSeed :type Integer))
  (bind _currentpointlocationsrelative (Variables|Default|GetCurrentPointLocationsRelative))
  (Utilities|FlowControl|Sequence
    (:then_0
      (Utilities|Array|SetArrayElem _currentpointlocationsrelative Point (+ (Utilities|Array|Get(acopy) _currentpointlocationsrelative Point) AddLocation))
      (CallFunction|SetWorldPositions))
    (:then_1
      (Variables|Default|SetWidth (Math|Float|Clamp(Float) (+ (Variables|Default|GetWidth) WidthChange) 2.7e+03 1e+04))
      (Variables|Default|SetCurrentSeed (Math|Integer|SelectInt NewSeed (Variables|Default|GetCurrentSeed) UseNewSeeed))
      (bind _asbp_procedural_cave (Utilities|Casting|CastToBP_ProceduralCave (Variables|/Script/Engine.ChildActorComponent|GetChildActor (Variables|Default|GetChildActor))))
      (Default|VariablesSetup _asbp_procedural_cave (Variables|Default|GetCurrentPointLocationsWorld) true (Variables|Default|GetMeshes) 1.0 (Variables|Default|GetCurrentSeed) false (Variables|Default|GetWidth) 0.35 "/Game/ProceduralCaves/Blueprints/Curves/ExampleCurve.ExampleCurve" true 2e+03 1 1 "/Game/ProceduralCaves/CustomMeshes/SM_HollowCylinderRough.SM_HollowCylinderRough" (Utilities|Array|MakeArray 0) "NoCollision" "ECC_WorldStatic" true 11.0 "(R=0.509804,G=0.415686,B=0.243137,A=1.000000)" 0.55 1.6 0.0 true))))

(fn Reset
  (Variables|Default|SetCurrentPointLocationsRelative (Utilities|Array|MakeArray "0,-1500.000000, 0" "15000.000000,-5000.000000,-1500.000000" "30000.000000,-2500.000000, 0"))
  (Variables|Default|SetWidth 5.5e+03)
  (Variables|Default|SetCurrentSeed 2)
  (CallFunction|SetWorldPositions)
  (bind _asbp_procedural_cave (Utilities|Casting|CastToBP_ProceduralCave (Variables|/Script/Engine.ChildActorComponent|GetChildActor (Variables|Default|GetChildActor))))
  (Default|VariablesSetup _asbp_procedural_cave (Variables|Default|GetCurrentPointLocationsWorld) true (Variables|Default|GetMeshes) 1.0 (Variables|Default|GetCurrentSeed) false (Variables|Default|GetWidth) 0.35 "/Game/ProceduralCaves/Blueprints/Curves/ExampleCurve.ExampleCurve" true 2e+03 1 1 "/Game/ProceduralCaves/CustomMeshes/SM_HollowCylinderRough.SM_HollowCylinderRough" (Utilities|Array|MakeArray 0) "NoCollision" "ECC_WorldStatic" true 11.0 "(R=0.509804,G=0.415686,B=0.243137,A=1.000000)" 0.55 1.6 0.0 true))

(fn SetWorldPositions
  (for (_array_element _array_index) (Variables|Default|GetCurrentPointLocationsRelative)
    (Utilities|Array|SetArrayElem (Variables|Default|GetCurrentPointLocationsWorld) _array_index (Math|Transform|InverseTransformLocation (Math|Transform|InvertTransform (Transformation|GetWorldTransform (Variables|Default|GetChildActor))) _array_element) true)))