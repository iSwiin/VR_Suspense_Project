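; Seeded randomization function library for procedural caves, returning repeatable bools, range-limited floats and rotators from an integer seed.
; StreamMaker scrambles the seed by using a first stream's random integer to seed a second, and each helper draws from such a fresh stream.
; The clamped rotator reuses one seed for all three axes, so roll, pitch and yaw land at the same relative point within their ranges.
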(fn RandomRotatorfromSeed
  (params (Seed :type Integer))
  (return (Class|KismetMathLibrary|RandomRotatorfromStream (CallFunction|StreamMaker Seed) true)))

(fn RandomClampedFloatfromSeed
  (params (Seed :type Integer) (Min :type Float%20%28single-precision%29) (Max :type Float%20%28single-precision%29))
  (return (Math|Random|RandomFloatinRangefromStream (CallFunction|StreamMaker Seed) Min Max)))

(fn RandomBoolfromSeed
  (params (Seed :type Integer))
  (return (Math|Random|RandomBoolfromStream (CallFunction|StreamMaker Seed))))

(fn StreamMaker
  (params (InitialSeed :type Integer))
  (return (Math|Random|MakeRandomStream (Class|KismetMathLibrary|RandomIntegerfromStream (Math|Random|MakeRandomStream InitialSeed) 99999999))))

(fn RandomClampedRotatorfromSeed
  (params (Seed :type Integer) (Min%20Rotation :type Rotator) (Max%20Rotation :type Rotator))
  (bind (_roll _pitch _yaw) (Math|Rotator|BreakRotator Max%20Rotation))
  (bind (_roll_2 _pitch_2 _yaw_2) (Math|Rotator|BreakRotator Min%20Rotation))
  (return (Math|Rotator|MakeRotator (CallFunction|RandomClampedFloatfromSeed Seed _roll_2 _roll) (CallFunction|RandomClampedFloatfromSeed Seed _pitch_2 _pitch) (CallFunction|RandomClampedFloatfromSeed Seed _yaw_2 _yaw))))