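; BP_TutorialWidgetActor is a placeable actor that shows tutorial text through a widget component.
; A shared Setup function casts the component's widget to WBP_TutorialWidget and passes it the actor's text, width and height overrides, and size.
; Setup runs from both the construction script and BeginPlay.
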(event EventBeginPlay
  (CallFunction|Setup))

(fn ConstructionScript
  (CallFunction|Setup))

(fn Setup
  (bind _aswbp_tutorial_widget (Utilities|Casting|CastToWBP_TutorialWidget (UserInterface|GetWidget (Variables|Default|GetWidget))))
  (Default|SetText _aswbp_tutorial_widget (Variables|Default|GetIn%20String) (Variables|Default|GetIn%20Height%20Override) (Variables|Default|GetIn%20Width%20Override) (Variables|Default|GetSize)))