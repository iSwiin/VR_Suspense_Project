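; Player pawn for the procedural caves project that drives its Demo and Tutorial levels.
; BeginPlay adds an info widget, then branches on level name: Demo adds a point controller widget and runs a hardware benchmark, while Tutorial sets fixed scalability.
; Number keys toggle the cursor and controller widget in Demo or switch levels.
; ServerChange rolls a seed and passes cave point edits or resets through MulticastChange to the target.
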(event Custom|ServerChange
  (params (RESET :type Boolean) (Target :type BP%20in%20Game%20Cave%20Handler%20Object%20Reference) (Point :type Integer) (AddLocation :type Vector) (WidthChange :type Float%20%28double-precision%29) (RandomSeed :type Boolean))
  (CallFunction|MulticastChange RESET Target Point AddLocation WidthChange RandomSeed (Math|Random|RandomIntegerinRange 0 9999)))

(event Custom|MulticastChange
  (params (RESET :type Boolean) (Target :type BP%20in%20Game%20Cave%20Handler%20Object%20Reference) (Point :type Integer) (AddLocation :type Vector) (WidthChange :type Float%20%28double-precision%29) (RandomSeed :type Boolean) (NewSeed :type Integer))
  (if (not RESET)
    (Default|Change Target Point AddLocation WidthChange RandomSeed NewSeed)
    (else
      (Default|Reset Target))))

(event EventBeginPlay
  (Development|ExecuteConsoleCommand "ShowFlag.Splines 1" 0)
  (bind _returnvalue (UserInterface|CreateWidget "/Game/ProceduralCaves/Blueprints/Widget_Blueprints/WBP_DemoOrTutorialWidget.WBP_DemoOrTutorialWidget_C"))
  (UserInterface|Viewport|AddtoViewport _returnvalue 12)
  (bind _returnvalue_2 (Game|GetCurrentLevelName true))
  (switch string _returnvalue_2
    (:Demo
      (bind _returnvalue_3 (UserInterface|CreateWidget "/Game/ProceduralCaves/Blueprints/Widget_Blueprints/WBP_PointController.WBP_PointController_C"))
      (bind _output_get (Variables|Default|SetwidgetTemp _returnvalue_3))
      (UserInterface|Viewport|AddtoViewport _output_get 0)
      (Default|StateChange (Variables|Default|GetwidgetTemp) true)
      (Input|SetInputModeUIOnly (Game|GetPlayerController 0) 0 "DoNotLock" false)
      (Variables|/Script/Engine.PlayerController|SetbShowMouseCursor (Game|GetPlayerController 0) true)
      (Utilities|FlowControl|Delay 0.1)
      (bind _returnvalue_4 (Settings|GetGameUserSettings))
      (Class|GameUserSettings|RunHardwareBenchmark _returnvalue_4 10 0.2 0.2)
      (Class|GameUserSettings|ApplyHardwareBenchmarkResults _returnvalue_4)
      (Utilities|FlowControl|Delay 1.0)
      (Input|SetInputModeGameandUI (Game|GetPlayerController 0) (Variables|Default|GetwidgetTemp) "DoNotLock" true false)
      (Default|StateChange (Variables|Default|GetwidgetTemp) false)
      (Development|ExecuteConsoleCommand "r.VSync 1" 0))
    (:Tutorial
      (Development|ExecuteConsoleCommand "SCALABILITY 2" 0)
      (Development|ExecuteConsoleCommand "r.VSync 1" 0))))

(event Input|KeyboardEvents|1
  (params (Key :type Key%20Structure))
  (bind _returnvalue (Game|GetPlayerController 0))
  (:Pressed
    (bind _returnvalue_2 (Game|GetCurrentLevelName true))
    (switch string _returnvalue_2
      (:Demo
        (bind _output_get (Variables|/Script/Engine.PlayerController|SetbShowMouseCursor (Game|GetPlayerController 0) (not (Variables|/Script/Engine.PlayerController|GetbShowMouseCursor (Game|GetPlayerController 0)))))
        (if _output_get
          (Input|SetInputModeGameandUI _returnvalue (Variables|Default|GetwidgetTemp) "DoNotLock" true false)
          (else
            (Input|SetInputModeGameOnly _returnvalue false)))))))

(event Input|KeyboardEvents|2
  (params (Key :type Key%20Structure))
  (bind _widgettemp (Variables|Default|GetwidgetTemp))
  (:Pressed
    (bind _returnvalue (Game|GetCurrentLevelName true))
    (switch string _returnvalue
      (:Demo
        (Utilities|FlowControl|FlipFlop
          (:A
            (Widget|SetVisibility _widgettemp "Hidden"))
          (:B
            (Widget|SetVisibility _widgettemp "Visible")))))))

(event Input|KeyboardEvents|8
  (params (Key :type Key%20Structure))
  (:Pressed
    (Game|OpenLevel(byName) "Demo")
    (Variables|/Script/Engine.PlayerController|SetbShowMouseCursor (Game|GetPlayerController 0) false)
    (Input|SetInputModeGameandUI (Game|GetPlayerController 0) (Variables|Default|GetwidgetTemp) "DoNotLock" true false)))

(event Input|KeyboardEvents|9
  (params (Key :type Key%20Structure))
  (:Pressed
    (Game|OpenLevel(byName) "Tutorial")
    (Variables|/Script/Engine.PlayerController|SetbShowMouseCursor (Game|GetPlayerController 0) false)
    (Input|SetInputModeGameOnly (Game|GetPlayerController 0) false)))

(fn ConstructionScript)